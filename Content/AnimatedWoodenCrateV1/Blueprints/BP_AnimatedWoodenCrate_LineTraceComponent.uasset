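; Player character component that lets a first-person camera interact with animated wooden crates by line trace.
; The interact input builds a trace from the owner's camera along its forward vector, limited by InteractionRange.
; A reliable server RPC, named for a dynamic campfire, relays the endpoints to a reliable multicast.
; Each machine then runs the Visibility trace itself and sends the crate interact message to the hit actor.
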(event Custom|Dynamic%20Campfire%20Line%20Trace%20Interaction:%20Run%20On%20Server
  (params (Start :type Vector) (End :type Vector))
  ;[0.3501 1 0.2964 1 45] Line Trace Interaction - Meant for BP_AnimatedWoodenCrate
  ;;[1 0.5373 0 1 30] Replication: Custom Events for the RPC (Remote Procedure Calls) necessary in multiplayer projects.
  ;;;[1 0.5373 0] Run On Server - Reliable
  (CallFunction|DynamicCampfireLineTraceInteraction:Multicast Start End))

(event Custom|Dynamic%20Campfire%20Line%20Trace%20Interaction:%20Multicast
  (params (Start :type Vector) (End :type Vector))
  ;[0.3501 1 0.2964 1 45] Line Trace Interaction - Meant for BP_AnimatedWoodenCrate
  ;;[1 0.5373 0 1 30] Replication: Custom Events for the RPC (Remote Procedure Calls) necessary in multiplayer projects.
  ;;;[1 0.5373 0] Multicast - Reliable
  (bind _outhit (Collision|LineTraceByChannel Start End "TraceTypeQuery1" false 0 "None"))
  (Class|BPIAnimatedWoodenCrateInteraction|AnimatedWoodenCrateInteract(Message) (.HitActor (Collision|BreakHitResult _outhit))))

(event Input|EnhancedActionEvents|EnhancedInputActionIA_InteractMouse1
  (params (ActionValue :type Boolean) (ElapsedSeconds :type Float%20%28double-precision%29) (TriggeredSeconds :type Float%20%28double-precision%29) (InputAction :type Input%20Action%20Object%20Reference :default "/Game/AnimatedWoodenCrateV1/DemoLevel/DemoCharacter/Input/Actions/IA_InteractMouse1.IA_InteractMouse1"))
  (bind _returnvalue (Components|GetOwner))
  (bind _returnvalue_2 (Actor|GetComponentbyClass _returnvalue "/Script/Engine.CameraComponent"))
  (bind _returnvalue_3 (Transformation|GetWorldLocation _returnvalue_2))
  ;[0.3501 1 0.2964 1 45] Line Trace Interaction - Meant for BP_AnimatedWoodenCrate
  ;;[0.3501 1 0.2964] Input Action Left Mouse Button
  (:Triggered
    ;;[1 0.5373 0 1 30] Replication: Custom Events for the RPC (Remote Procedure Calls) necessary in multiplayer projects.
    (CallFunction|DynamicCampfireLineTraceInteraction:RunonServer _returnvalue_3 (+ _returnvalue_3 (* (Math|Vector|GetForwardVector _returnvalue_2) (Variables|Default|GetInteraction%20Range))))))