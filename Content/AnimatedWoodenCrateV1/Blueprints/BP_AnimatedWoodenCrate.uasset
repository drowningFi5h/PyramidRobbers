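; BP_AnimatedWoodenCrate is an interactable wooden crate that toggles between open and closed.
; Its interact event plays the matching skeletal animation and audio component, then flips the Open flag.
; A DoOnce, reset after a short delay, acts as an interaction cooldown.
; The construction script applies a configurable static mesh and relative transform to the crate's content component.
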(event EventAnimatedWoodenCrateInteract
  (bind _woodencrate (Variables|Default|GetWoodenCrate))
  (bind _audioopen (Variables|Default|GetAudioOpen))
  (bind _audioclose (Variables|Default|GetAudioClose))
  (Utilities|FlowControl|DoOnce false :!label _label ; Interaction Cooldown
    (:Completed
      (Utilities|FlowControl|Sequence
        (:then_0
          (if (Variables|WoodenCrateState|GetOpen)
            (Components|Animation|PlayAnimation _woodencrate "/Game/AnimatedWoodenCrateV1/Animations/AS_WoodenCrateClose.AS_WoodenCrateClose" false)
            (Audio|Components|Audio|SetVolumeMultiplier _audioclose 1.0 :!class /Script/Engine.AudioComponent)
            (Audio|Components|Audio|Play _audioclose 0.0)
            (Variables|WoodenCrateState|SetOpen false)
            (else
              (Components|Animation|PlayAnimation _woodencrate "/Game/AnimatedWoodenCrateV1/Animations/AS_WoodenCrateOpen.AS_WoodenCrateOpen" false)
              (Audio|Components|Audio|SetVolumeMultiplier _audioopen 1.0 :!class /Script/Engine.AudioComponent)
              (Audio|Components|Audio|Play _audioopen 0.0)
              (Variables|WoodenCrateState|SetOpen true))))
        (:then_1
          (Utilities|FlowControl|Delay 0.5)
          (goto _label Reset))))))

(fn ConstructionScript
  (Components|StaticMesh|SetStaticMesh (Variables|Default|GetWoodenCrateContent) (Variables|WoodenCrateContentProperties|GetWoodenCrateContentMesh))
  (Transformation|SetRelativeTransform (Variables|Default|GetWoodenCrateContent) (Math|Transform|MakeTransform (Variables|WoodenCrateContentProperties|GetContentLocation) (Variables|WoodenCrateContentProperties|GetContentRotation) (Variables|WoodenCrateContentProperties|GetContentScale)) false false))